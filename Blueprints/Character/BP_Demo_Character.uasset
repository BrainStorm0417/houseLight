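; First-person demo character that walks, looks around and interacts with furniture.
; WASD keys set direction values that Tick feeds into movement input, while mouse axes drive yaw and inverted pitch.
; Each Tick, a short camera line trace toggles the crosshair widget on components tagged "Active" and sends a trace message to the hit actor.
; Pressing E sends that actor an action message with the hit component.
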(event EventBeginPlay
  ;[1 1 1] Event Begin Play
  (bind _returnvalue (UserInterface|CreateWidget "/Game/HouseFurniture/Blueprints/Character/BP_CrossPoint.BP_CrossPoint_C"))
  (bind _output_get (Variables|Default|SetCrossPointWidget _returnvalue))
  (UserInterface|Viewport|AddtoViewport _output_get 0))

(event EventTick
  (params (DeltaSeconds :type Float%20%28single-precision%29))
  (bind _camera (Variables|Default|GetCamera))
  (bind _crosspointwidget (Variables|Default|GetCrossPointWidget))
  (bind _returnvalue (Transformation|GetWorldLocation _camera))
  (Utilities|FlowControl|Sequence
    (:then_0
      ;[1 1 1] MovementPart
      (Pawn|Input|AddMovementInput (+ (* (Transformation|GetActorForwardVector) (Variables|Default|GetMoveForward)) (* (Transformation|GetActorRightVector) (Variables|Default|GetMoveRight))) 1.0 false))
    (:then_1
      ;[1 1 1] TracePart
      (bind _outhit (Collision|LineTraceByChannel _returnvalue (+ _returnvalue (* (Math|Vector|GetForwardVector _camera) 2.5e+02)) "TraceTypeQuery1" false 0 "None" true "(R=0.000000,G=1.000000,B=0.000000,A=1.000000)"))
      (Variables|Default|SetTraceResult _outhit)
      (if (Utilities|IsValid (.HitActor (Collision|BreakHitResult (Variables|Default|GetTraceResult))))
        (if (Components|ComponentHasTag (.HitComponent (Collision|BreakHitResult (Variables|Default|GetTraceResult))) "Active")
          (Default|SwithCrossPoint _crosspointwidget true)
          (else
            (Default|SwithCrossPoint _crosspointwidget false :!label _label)))
        (else
          (goto _label)))
      (Class|BPDemoInterface|FurnitureTrace(Message) (.HitActor (Collision|BreakHitResult (Variables|Default|GetTraceResult)))))))

(event Input|MouseEvents|MouseY
  (params (AxisValue :type Float%20%28single-precision%29))
  ;[1 1 1] MouseInput
  (Pawn|Input|AddControllerPitchInput (* AxisValue -1.0)))

(event Input|MouseEvents|MouseX
  (params (AxisValue :type Float%20%28single-precision%29))
  ;[1 1 1] MouseInput
  (Pawn|Input|AddControllerYawInput AxisValue))

(event Input|KeyboardEvents|D
  (params (Key :type Key%20Structure))
  ;[1 1 1] MovementInput
  (:Pressed
    (Variables|Default|SetMoveRight 1))
  (:Released
    (if (== (Variables|Default|GetMoveRight) 1)
      (Variables|Default|SetMoveRight 0))))

(event Input|KeyboardEvents|A
  (params (Key :type Key%20Structure))
  ;[1 1 1] MovementInput
  (:Pressed
    (Variables|Default|SetMoveRight -1))
  (:Released
    (if (== (Variables|Default|GetMoveRight) -1)
      (Variables|Default|SetMoveRight 0))))

(event Input|KeyboardEvents|E
  (params (Key :type Key%20Structure))
  (bind _traceresult (Variables|Default|GetTraceResult))
  (bind (_bblockinghit _binitialoverlap _time _distance _location _impactpoint _normal _impactnormal _physmat _hitactor _hitcomponent) (Collision|BreakHitResult _traceresult))
  ;[1 1 1] InteractionPart
  (:Pressed
    (Class|BPDemoInterface|FurnitureAction(Message) _hitactor _hitcomponent)))

(event Input|KeyboardEvents|W
  (params (Key :type Key%20Structure))
  ;[1 1 1] MovementInput
  (:Pressed
    (Variables|Default|SetMoveForward 1))
  (:Released
    (if (== (Variables|Default|GetMoveForward) 1)
      (Variables|Default|SetMoveForward 0))))

(event Input|KeyboardEvents|S
  (params (Key :type Key%20Structure))
  ;[1 1 1] MovementInput
  (:Pressed
    (Variables|Default|SetMoveForward -1))
  (:Released
    (if (== (Variables|Default|GetMoveForward) -1)
      (Variables|Default|SetMoveForward 0))))

(fn ConstructionScript)